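; Enemy AI controller that makes its controlled pawn chase the first player's pawn.
; A looping timer started on BeginPlay repeatedly sets focus on the player and issues an AI MoveTo toward it, stopping on overlap.
; If the player pawn is invalid, it stops movement and clears focus; debug prints report move results and the invalid case.
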(event Custom|TickMoveToPlayer
  (bind _returnvalue (Game|Player|GetPlayerPawn 0))
  (if (Utilities|IsValid _returnvalue)
    (AI|SetFocus _returnvalue)
    (AI|AIMoveTo (Pawn|GetControlledPawn) "0, 0, 0" _returnvalue 5.0 true
      (:OnSuccess
        (Development|PrintString "AIMoveToSuccess"))
      (:OnFail
        (Development|PrintString "AIMoveToFail")))
    (else
      (AI|Navigation|StopMovement)
      (AI|ClearFocus)
      (Development|PrintString "invalid player"))))

(event EventBeginPlay
  (Utilities|Time|SetTimerbyEvent (delegate Custom|TickMoveToPlayer) 0.25 true))

(fn ConstructionScript)